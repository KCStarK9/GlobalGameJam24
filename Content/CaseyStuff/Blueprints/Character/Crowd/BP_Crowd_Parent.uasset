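; BP_Crowd_Parent is a crowd character Blueprint whose Paper2D flipbook animates in response to the game's hype level.
; On BeginPlay it rolls a random hype threshold and binds GETHYPE to the hype update from BP_JamGameMode.
; Each update compares the current-to-required hype ratio with that threshold, either scaling the flipbook play rate with the ratio or freezing it below the threshold.
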(event `self.ReceiveBeginPlay`
  (set `self.HypeThreshold` (`KismetMathLibrary.RandomFloatInRange` 0.1 0.8))
  (bind _asbp_jam_game_mode (cast `/Game/CaseyStuff/Blueprints/BP_JamGameMode` (`GameplayStatics.GetGameMode`)))
  (bind _output_get (set `self.Game Mode Ref` _asbp_jam_game_mode))
  (add `/Game/CaseyStuff/Blueprints/BP_JamGameMode.HypeUpdate` _output_get (delegate `GET HYPE`)))

(event `GET HYPE`
  (bind _game_mode_ref (`self.Game Mode Ref`))
  (bind _paperflipbook (`self.PaperFlipbook`))
  (bind _returnvalue (/ (`KismetMathLibrary.Conv_IntToDouble` (`/Game/CaseyStuff/Blueprints/BP_JamGameMode.CurrentHype` _game_mode_ref)) (`KismetMathLibrary.Conv_IntToDouble` (`/Game/CaseyStuff/Blueprints/BP_JamGameMode.RequiredHype` _game_mode_ref))))
  (if (>= _returnvalue (`self.HypeThreshold`))
    (`PaperFlipbookComponent.SetPlayRate` _paperflipbook (`KismetMathLibrary.Lerp` 0.0 3.0 _returnvalue))
    (else
      (`PaperFlipbookComponent.SetPlayRate` _paperflipbook 0.0))))

(fn `UserConstructionScript`)