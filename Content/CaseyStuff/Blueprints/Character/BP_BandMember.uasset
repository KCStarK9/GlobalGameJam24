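; BP_BandMember is a band member in the jam game, playing sound and animating to the crowd's hype.
; On BeginPlay it binds to BP_JamGameMode's start-sound and hype-update events.
; Start-sound spawns a random 2D sound through a DoOnce, which resets only for the Vocalist so that member can trigger again.
; Hype updates scale the Paper flipbook's play rate by the ratio of current to required hype.
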(event `StartSound`
  (`/Engine/EditorBlueprintResources/StandardMacros.DoOnce` false :!label _label
    (:`Completed`
      (`GameplayStatics.SpawnSound2D` (`KismetArrayLibrary.Array_Random` (`self.Sound`)) 1.0 1.0 0.0 null false false)
      (if (== (`self.MemberType`) "Vocalist")
        (goto _label :!via `Reset`)))))

(event `self.ReceiveBeginPlay`
  (bind _asbp_jam_game_mode (cast `/Game/CaseyStuff/Blueprints/BP_JamGameMode` (`GameplayStatics.GetGameMode`)))
  (bind _output_get (set `self.GameMode` _asbp_jam_game_mode))
  (add `/Game/CaseyStuff/Blueprints/BP_JamGameMode.StartSound` _output_get (delegate `StartSound`))
  (add `/Game/CaseyStuff/Blueprints/BP_JamGameMode.HypeUpdate` _output_get (delegate `GETHYPED`)))

(event `GETHYPED`
  (bind _gamemode (`self.GameMode`))
  (`PaperFlipbookComponent.SetPlayRate` (`self.PaperFlipbook`) (`KismetMathLibrary.Lerp` 0.0 5.0 (/ (`/Game/CaseyStuff/Blueprints/BP_JamGameMode.CurrentHype` _gamemode) (`/Game/CaseyStuff/Blueprints/BP_JamGameMode.RequiredHype` _gamemode)))))

(fn `UserConstructionScript`)