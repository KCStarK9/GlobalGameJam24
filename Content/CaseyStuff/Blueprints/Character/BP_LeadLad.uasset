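; BP_LeadLad is a character Blueprint whose Paper2D flipbook animation speed responds to the game's hype level.
; On BeginPlay it caches BP_JamGameMode and binds GETHYPED to that mode's hype update event.
; Each update sets the flipbook play rate with a Lerp driven by required hype divided by current hype, so playback slows as current hype rises relative to required.
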(event `self.ReceiveBeginPlay`
  (bind _asbp_jam_game_mode (cast `/Game/CaseyStuff/Blueprints/BP_JamGameMode` (`GameplayStatics.GetGameMode`)))
  (bind _output_get (set `self.GameMode` _asbp_jam_game_mode))
  (add `/Game/CaseyStuff/Blueprints/BP_JamGameMode.HypeUpdate` _output_get (delegate `GETHYPED`)))

(event `GETHYPED`
  (bind _gamemode (`self.GameMode`))
  (`PaperFlipbookComponent.SetPlayRate` (`self.PaperFlipbook`) (`KismetMathLibrary.Lerp` 0.0 5.0 (/ (`/Game/CaseyStuff/Blueprints/BP_JamGameMode.RequiredHype` _gamemode) (`/Game/CaseyStuff/Blueprints/BP_JamGameMode.CurrentHype` _gamemode)))))

(fn `UserConstructionScript`)