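; Game mode for a band-themed deck-building card game, running the deck, hand, discard pile and scoring.
; BeginPlay shuffles the game instance's deck and repeats a start-sound call every six seconds; draws recycle discards when the deck empties.
; Played cards add Hype, Groove or Epicness, draw, then get discarded, or just leave the hand if upgrades.
; Groove boosts positive Hype gains, while Epicness multiplies any Hype change and then resets.
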(event `self.ReceiveBeginPlay`
  (bind _returnvalue (`GameplayStatics.GetPlayerController` 0))
  (bind _asbp_jam_hud (cast `/Game/CaseyStuff/Blueprints/BP_JamHUD` (`PlayerController.GetHUD` _returnvalue)))
  (set `self.HUD` _asbp_jam_hud)
  (bind _asbp_jam_controller (cast `/Game/CaseyStuff/Blueprints/BP_JamController` _returnvalue))
  (set `self.PlayerController` _asbp_jam_controller)
  (bind _asbp_jam_instance (cast `/Game/CaseyStuff/Blueprints/BP_JamInstance` (`GameplayStatics.GetGameInstance`)))
  (bind _output_get (set `self.GameInstance` _asbp_jam_instance))
  (bind _output_get_2 (set `self.Deck` (`/Game/CaseyStuff/Blueprints/BP_JamInstance.CurrentDeck` _output_get)))
  (`KismetArrayLibrary.Array_Shuffle` _output_get_2)
  (`self.HypeUpdate`)
  (`KismetSystemLibrary.Delay` 6.0 :!label _label)
  (`self.StartSound`)
  (goto _label))

(event `GetHype`
  (params (HypeGain :type Integer))
  (bind _currenthype (`self.CurrentHype`))
  (bind _currenthype_2 (`self.CurrentHype`))
  (bind _returnvalue (+ HypeGain (`self.CurrentGroove`)))
  (if (< HypeGain 0)
    (if (== (`self.CurrentEpicness`) 0)
      (set `self.CurrentHype` (+ _currenthype_2 HypeGain))
      (else
        (set `self.CurrentHype` (+ _currenthype_2 (* HypeGain (* (`self.CurrentEpicness`) 2))))))
    (elif (== (`self.CurrentEpicness`) 0)
      (set `self.CurrentHype` (+ _currenthype _returnvalue))
      (else
        (set `self.CurrentHype` (+ _currenthype (* _returnvalue (* (`self.CurrentEpicness`) 2)))))))
  (set `self.CurrentEpicness` 0)
  (if (< (`self.CurrentHype`) 0)
    (set `self.CurrentHype` 0))
  (`self.HypeUpdate`))

(event `GetGroove`
  (params (GrooveGain :type Integer))
  (set `self.CurrentGroove` (+ (`self.CurrentGroove`) GrooveGain)))

(event `GainEpicness`
  (params (EpicGain :type Integer))
  (set `self.CurrentEpicness` (+ (`self.CurrentEpicness`) EpicGain)))

(event `Draw`
  (bind _hand (`self.Hand`))
  (bind _discardpile (`self.DiscardPile`))
  (bind _deck (`self.Deck`))
  (bind _deck_2 (`self.Deck`))
  (if (<= (`KismetArrayLibrary.Array_Length` _deck_2) 0)
    (for (_array_element _array_index) _discardpile
      (`KismetArrayLibrary.Array_Add` _deck _array_element)
      (`KismetArrayLibrary.Array_Remove` _discardpile _array_index))
    (`KismetArrayLibrary.Array_Shuffle` _deck)
    (`KismetSystemLibrary.Delay` 0.2))
  (bind _returnvalue (`KismetArrayLibrary.Array_Add` _hand (`|GetArrayItem` _deck_2)))
  (`KismetArrayLibrary.Array_Remove` _deck_2)
  (`/Game/CaseyStuff/Blueprints/BP_JamHUD.Hand_Add` (`self.HUD`) (`|GetArrayItem` _hand _returnvalue)))

(event `EndTurn`
  (for _array_element (`self.Hand`)
    (`self.Discard` _array_element)))

(event `CardPlay`
  (params (PlayedCard :type "/Game/CaseyStuff/Blueprints/S_Cards Structure"))
  (bind (_cardname _cardtext _cardimage _upgrade _bandmembertype _value _ishype _isgroove _isepicness _hypevalue _groovevalue _epicvalue _drawscard _drawamount) (break `/Game/CaseyStuff/Blueprints/S_Cards` PlayedCard))
  (`|ExecutionSequence`
    (:`then_0`
      (if _ishype
        (`self.GetHype` _hypevalue)))
    (:`then_1`
      (if _isgroove
        (`self.GetGroove` _groovevalue)))
    (:`then_2`
      (if _isepicness
        (`self.GainEpicness` _epicvalue)))
    (:`then_3`
      (if _drawscard
        (bind _counter (`/Engine/EditorBlueprintResources/StandardMacros.Do N` _drawamount :!label _label_2)
          (:`Exit`
            (`self.Draw`)
            (`KismetSystemLibrary.Delay` 0.2)
            (if (== 0 _counter)
              (goto _label_2 :!via `Reset`)
              (else
                (goto _label_2)))))))
    (:`then_4`
      (if _upgrade
        (`KismetArrayLibrary.Array_RemoveItem` (`self.Hand`) PlayedCard)
        (`/Game/CaseyStuff/Blueprints/BP_JamHUD.Hand_Remove` (`self.HUD`) PlayedCard)
        (else
          (`self.Discard` PlayedCard))))))

(event `self.ReceiveTick`
  (params (DeltaSeconds :type "Float (single-precision)"))
  (`self.HandUpdate`))

(event `Discard`
  (params (CardToDiscard :type "/Game/CaseyStuff/Blueprints/S_Cards Structure"))
  (bind _hand (`self.Hand`))
  (for (_array_element _array_index) _hand
    (if (== (`.CardName_8_389C0EC14E504F269FD16985D91252CE` (break `/Game/CaseyStuff/Blueprints/S_Cards` CardToDiscard)) (break `/Game/CaseyStuff/Blueprints/S_Cards` _array_element))
      (`KismetArrayLibrary.Array_Remove` _hand _array_index)
      (break)))
  (`KismetArrayLibrary.Array_Add` (`self.DiscardPile`) CardToDiscard)
  (`/Game/CaseyStuff/Blueprints/BP_JamHUD.Hand_Remove` (`self.HUD`) CardToDiscard))

(event `AddBandMember`
  (params (MemberToAdd :type Name)))

(fn `UserConstructionScript`)