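; BP_JamInstance is the game instance that holds the player's card deck and level progression.
; On Init it builds CurrentDeck from DT_Cards rows, using a self-looping DoN to add repeated PowerChord copies, then a single Gaz.
; A final loop over the deck does nothing, as its debug print is disconnected.
; NextLevel increments LevelSelect and opens that entry in Levels by name.
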(event `self.ReceiveInit`
  (bind _currentdeck (`self.CurrentDeck`))
  (`|ExecutionSequence`
    (:`then_0`
      (bind _returnvalue (`|GetDataTableRow` "/Game/CaseyStuff/Blueprints/DT_Cards.DT_Cards" "PowerChord")
        (:`then`
          (`/Engine/EditorBlueprintResources/StandardMacros.Do N` 5 :!label _label
            (:`Exit`
              (`KismetArrayLibrary.Array_Add` _currentdeck _returnvalue)
              (goto _label))))))
    (:`then_1`
      (bind _returnvalue_2 (`|GetDataTableRow` "/Game/CaseyStuff/Blueprints/DT_Cards.DT_Cards" "Gaz")
        (:`then`
          (`KismetArrayLibrary.Array_Add` _currentdeck _returnvalue_2))))
    (:`then_2`
      (for _array_element (`self.CurrentDeck`)
        _))))

(event `NextLevel`
  (bind _output_get (set `self.Level_Select` (+ (`self.Level_Select`) 1)))
  (`GameplayStatics.OpenLevel` (`|GetArrayItem` (`self.Levels`) _output_get)))