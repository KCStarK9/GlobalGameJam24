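; BP_JamController is the player controller for a jam game, currently a small setup skeleton.
; On BeginPlay, if the Enhanced Input subsystem is valid, it adds the IMC_Jam mapping context, then caches typed references to the jam game mode, HUD and game instance.
; The casts run in sequence, so a failed one skips the rest.
; The Hello input action only prints a test message.
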(event `self.ReceiveBeginPlay`
  (bind _returnvalue (pcsubsystem `EnhancedInputLocalPlayerSubsystem` self))
  (`/Engine/EditorBlueprintResources/StandardMacros.IsValid` _returnvalue
    (:`Is Valid`
      (`EnhancedInputSubsystemInterface.AddMappingContext` _returnvalue "/Game/CaseyStuff/Blueprints/Inputs/IMC_Jam.IMC_Jam" 0 (struct))
      (bind _asbp_jam_game_mode (cast `/Game/CaseyStuff/Blueprints/BP_JamGameMode` (`GameplayStatics.GetGameMode`)))
      (set `self.GameMode` _asbp_jam_game_mode)
      (bind _asbp_jam_hud (cast `/Game/CaseyStuff/Blueprints/BP_JamHUD` (`self.GetHUD`)))
      (set `self.HUD` _asbp_jam_hud)
      (bind _asbp_jam_instance (cast `/Game/CaseyStuff/Blueprints/BP_JamInstance` (`GameplayStatics.GetGameInstance`)))
      (set `self.GameInstance` _asbp_jam_instance))))

(event `EnhancedInput|/Game/CaseyStuff/Blueprints/Inputs/Hello`
  (params (ActionValue :type Boolean) (ElapsedSeconds :type "Float (double-precision)") (TriggeredSeconds :type "Float (double-precision)") (InputAction :type "InputAction Object Reference" :default "/Game/CaseyStuff/Blueprints/Inputs/Hello.Hello"))
  (:`Started`
    (`KismetSystemLibrary.PrintString` "Hello")))

(fn `UserConstructionScript`)